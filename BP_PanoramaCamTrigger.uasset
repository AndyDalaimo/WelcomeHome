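; BP_PanoramaCamTrigger is a trigger volume that switches the player's view to its own camera while BP_Player stands inside its box.
; BeginPlay caches the player actor, and box overlap begin sets the view target to this actor and shows the Door component.
; Overlap end returns the view to the player and hides the Door again.
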(event OnComponentBeginOverlap(Box)
  (params (OverlappedComponent :type Primitive%20Component%20Object%20Reference) (OtherActor :type Actor%20Object%20Reference) (OtherComp :type Primitive%20Component%20Object%20Reference) (OtherBodyIndex :type Integer) (bFromSweep :type Boolean) (SweepResult :type Hit%20Result%20Structure%20%28by%20ref%29))
  (if (== OtherActor (Variables|Default|GetPlayerRef))
    (Game|Player|SetViewTargetwithBlend (Game|GetPlayerController (Game|GetPlayerState 0)) self 0.0 "VTBlend_Linear" 0.0 false)
    (Rendering|SetVisibility (Variables|Default|GetDoor) true false)))

(event OnComponentEndOverlap(Box)
  (params (OverlappedComponent :type Primitive%20Component%20Object%20Reference) (OtherActor :type Actor%20Object%20Reference) (OtherComp :type Primitive%20Component%20Object%20Reference) (OtherBodyIndex :type Integer))
  (if (== OtherActor (Variables|Default|GetPlayerRef))
    (Game|Player|SetViewTargetwithBlend (Game|GetPlayerController (Game|GetPlayerState 0)) (Variables|Default|GetPlayerRef) 0.0 "VTBlend_Linear" 0.0 false)
    (if (Variables|/Script/Engine.SceneComponent|GetbVisible (Variables|Default|GetDoor))
      (Rendering|SetVisibility (Variables|Default|GetDoor) false false))))

(event EventBeginPlay
  (bind _returnvalue (Actor|GetActorOfClass "/Game/Player/Blueprints/BP_Player.BP_Player_C"))
  (Variables|Default|SetPlayerRef _returnvalue))

(fn ConstructionScript)